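; BP_Buildings is a runner-game environment segment that fills itself with randomly chosen buildings.
; Its construction script runs SpawnBuildings, which makes a random eleven-way pick for each of four spawn points and adds a child actor there.
; Overlapping its Box calls ExtendBuildings on BP_RunnerGameMode to extend the environment.
; GetAttachPoint returns the Arrow's world transform, exposing an attach point for the segment.
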(event OnComponentBeginOverlap(Box)
  (params (OverlappedComponent :type Primitive%20Component%20Object%20Reference) (OtherActor :type Actor%20Object%20Reference) (OtherComp :type Primitive%20Component%20Object%20Reference) (OtherBodyIndex :type Integer) (bFromSweep :type Boolean) (SweepResult :type Hit%20Result%20Structure%20%28by%20ref%29))
  ;[1 0.867 0] ExtendEnvironment
  (bind _asbp_runner_game_mode (Utilities|Casting|CastToBP_RunnerGameMode (Game|GetGameMode)))
  (Default|ExtendBuildings _asbp_runner_game_mode))

(event EventBeginPlay)

(event EventTick
  (params (DeltaSeconds :type Float%20%28single-precision%29)))

(fn ConstructionScript
  (CallFunction|SpawnBuildings))

(fn GetAttachPoint
  (return (Transformation|GetWorldTransform (Variables|Default|GetArrow))))

(fn SpawnBuildings
  (bind _sp1 (Variables|Default|GetSP1))
  (bind _sp2 (Variables|Default|GetSP2))
  (bind _sp3 (Variables|Default|GetSP3))
  (bind _sp4 (Variables|Default|GetSP4))
  (bind _returnvalue (Transformation|GetRelativeTransform _sp3))
  (bind _returnvalue_2 (Transformation|GetRelativeTransform _sp4))
  (bind _returnvalue_3 (Transformation|GetRelativeTransform _sp1))
  (bind _returnvalue_4 (Transformation|GetRelativeTransform _sp2))
  (Utilities|FlowControl|Sequence
    (:then_0
      (switch int (Math|Random|RandomIntegerinRange 0 10)
        (:0
          (AddComponent|AddChildActorComponent false _returnvalue_3))
        (:1
          (AddComponent|AddChildActorComponent false _returnvalue_3))
        (:2
          (AddComponent|AddChildActorComponent false _returnvalue_3))
        (:3
          (AddComponent|AddChildActorComponent false _returnvalue_3))
        (:4
          (AddComponent|AddChildActorComponent false _returnvalue_3))
        (:5
          (AddComponent|AddChildActorComponent false _returnvalue_3))
        (:6
          (AddComponent|AddChildActorComponent false _returnvalue_3))
        (:7
          (AddComponent|AddChildActorComponent false _returnvalue_3))
        (:8
          (AddComponent|AddChildActorComponent false _returnvalue_3))
        (:9
          (AddComponent|AddChildActorComponent false _returnvalue_3))
        (:10
          (AddComponent|AddChildActorComponent false _returnvalue_3))))
    (:then_1
      (switch int (Math|Random|RandomIntegerinRange 0 10)
        (:0
          (AddComponent|AddChildActorComponent false _returnvalue_4))
        (:1
          (AddComponent|AddChildActorComponent false _returnvalue_4))
        (:2
          (AddComponent|AddChildActorComponent false _returnvalue_4))
        (:3
          (AddComponent|AddChildActorComponent false _returnvalue_4))
        (:4
          (AddComponent|AddChildActorComponent false _returnvalue_4))
        (:5
          (AddComponent|AddChildActorComponent false _returnvalue_4))
        (:6
          (AddComponent|AddChildActorComponent false _returnvalue_4))
        (:7
          (AddComponent|AddChildActorComponent false _returnvalue_4))
        (:8
          (AddComponent|AddChildActorComponent false _returnvalue_4))
        (:9
          (AddComponent|AddChildActorComponent false _returnvalue_4))
        (:10
          (AddComponent|AddChildActorComponent false _returnvalue_4))))
    (:then_2
      (switch int (Math|Random|RandomIntegerinRange 0 10)
        (:0
          (AddComponent|AddChildActorComponent false _returnvalue))
        (:1
          (AddComponent|AddChildActorComponent false _returnvalue))
        (:2
          (AddComponent|AddChildActorComponent false _returnvalue))
        (:3
          (AddComponent|AddChildActorComponent false _returnvalue))
        (:4
          (AddComponent|AddChildActorComponent false _returnvalue))
        (:5
          (AddComponent|AddChildActorComponent false _returnvalue))
        (:6
          (AddComponent|AddChildActorComponent false _returnvalue))
        (:7
          (AddComponent|AddChildActorComponent false _returnvalue))
        (:8
          (AddComponent|AddChildActorComponent false _returnvalue))
        (:9
          (AddComponent|AddChildActorComponent false _returnvalue))
        (:10
          (AddComponent|AddChildActorComponent false _returnvalue))))
    (:then_3
      (switch int (Math|Random|RandomIntegerinRange 0 10)
        (:0
          (AddComponent|AddChildActorComponent false _returnvalue_2))
        (:1
          (AddComponent|AddChildActorComponent false _returnvalue_2))
        (:2
          (AddComponent|AddChildActorComponent false _returnvalue_2))
        (:3
          (AddComponent|AddChildActorComponent false _returnvalue_2))
        (:4
          (AddComponent|AddChildActorComponent false _returnvalue_2))
        (:5
          (AddComponent|AddChildActorComponent false _returnvalue_2))
        (:6
          (AddComponent|AddChildActorComponent false _returnvalue_2))
        (:7
          (AddComponent|AddChildActorComponent false _returnvalue_2))
        (:8
          (AddComponent|AddChildActorComponent false _returnvalue_2))
        (:9
          (AddComponent|AddChildActorComponent false _returnvalue_2))
        (:10
          (AddComponent|AddChildActorComponent false _returnvalue_2))))))