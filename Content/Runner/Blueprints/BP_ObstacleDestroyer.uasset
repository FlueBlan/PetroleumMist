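; BP_ObstacleDestroyer is a runner-game actor that removes blocker and wall obstacles it overlaps while the player character is dead.
; On begin overlap it reads IsDead from the player's BP_RunnerCharacter and destroys itself immediately if the player is alive.
; Otherwise it casts the overlapping actor to each obstacle class, destroys a match, then destroys itself after a short delay.
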(event Collision|EventActorBeginOverlap
  (params (OtherActor :type Actor%20Object%20Reference))
  (bind _asbp_runner_character (Utilities|Casting|CastToBP_RunnerCharacter (Game|GetPlayerCharacter 0)))
  (if (Variables|/Game/Runner/Blueprints/CharacterBPs/BP_RunnerCharacter.BP_RunnerCharacter_C|GetIsDead _asbp_runner_character)
    (Utilities|FlowControl|Sequence
      (:then_0
        (bind _asbp_obstacles_blocker (Utilities|Casting|CastToBP_Obstacles_Blocker OtherActor))
        (Actor|DestroyActor _asbp_obstacles_blocker))
      (:then_1
        (bind _asbp_obstacles_wall (Utilities|Casting|CastToBP_Obstacles_Wall OtherActor))
        (Actor|DestroyActor _asbp_obstacles_wall)))
    (Utilities|FlowControl|Delay 1.0)
    (Actor|DestroyActor)
    (else
      (Actor|DestroyActor))))

(fn ConstructionScript)