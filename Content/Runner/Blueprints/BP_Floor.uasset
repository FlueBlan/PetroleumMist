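; Endless-runner floor tile that fills its lanes with random obstacles, coins and occasional crates.
; Construction script builds per-lane arrow grids as spawn points, then shuffles them to place child actors.
; A crate spawns only once the game mode's FloorCount exceeds a threshold, which resets the count.
; Box overlap asks BP_RunnerGameMode to extend the floor, raises the player's clamped walk speed and adds multiplier-based points.
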(event OnComponentBeginOverlap(Box)
  (params (OverlappedComponent :type Primitive%20Component%20Object%20Reference) (OtherActor :type Actor%20Object%20Reference) (OtherComp :type Primitive%20Component%20Object%20Reference) (OtherBodyIndex :type Integer) (bFromSweep :type Boolean) (SweepResult :type Hit%20Result%20Structure%20%28by%20ref%29))
  ;[1 0.867 0] ExtendFloor
  (bind _asbp_runner_game_mode (Utilities|Casting|CastToBP_RunnerGameMode (Game|GetGameMode)))
  (Default|ExtendFloor _asbp_runner_game_mode)
  ;[0 1 0.07398] ChangeSpeed
  (bind _asbp_runner_character (Utilities|Casting|CastToBP_RunnerCharacter (Game|GetPlayerCharacter 0)))
  (bind _output_get (Variables|/Script/Engine.CharacterMovementComponent|SetMaxWalkSpeed (Variables|/Script/Engine.Character|GetCharacterMovement _asbp_runner_character) (Math|Float|Clamp(Float) (* (Variables|/Script/Engine.CharacterMovementComponent|GetMaxWalkSpeed (Variables|/Script/Engine.Character|GetCharacterMovement _asbp_runner_character)) 1.005) 7e+02 1.5e+03)))
  (Development|PrintString (Utilities|String|ToString(Float) _output_get))
  ;[0 1 0.7882] SetCurrentScore
  (bind _asbp_runner_game_mode_2 (Utilities|Casting|CastToBP_RunnerGameMode (Game|GetGameMode)))
  (Variables|/Game/Runner/Blueprints/BP_RunnerGameMode.BP_RunnerGameMode_C|SetCurrentPoints _asbp_runner_game_mode_2 (+ (* (Variables|/Game/Runner/Blueprints/BP_RunnerGameMode.BP_RunnerGameMode_C|GetPointsMult _asbp_runner_game_mode_2) 1) (Variables|/Game/Runner/Blueprints/BP_RunnerGameMode.BP_RunnerGameMode_C|GetCurrentPoints _asbp_runner_game_mode_2))))

(event EventBeginPlay)

(event EventTick
  (params (DeltaSeconds :type Float%20%28single-precision%29)))

(fn ConstructionScript
  (CallFunction|SetupSpawnPoints)
  (CallFunction|SpawnObstacles)
  (CallFunction|SpawnCoins)
  (CallFunction|CoinSpawner)
  (CallFunction|SpawnCrate)
  (CallFunction|CrateSpawner))

(fn GetAttachPoint
  (return (Transformation|GetWorldTransform (Variables|Default|GetArrow))))

(fn SetupSpawnPoints
  (for _array_element (Variables|Default|GetLanePosition)
    (for _index (range 0 1)
      (bind _returnvalue (AddComponent|AddArrowComponent false (Math|Transform|MakeTransform (Math|Vector|MakeVector (* _index 6e+02) _array_element 0.0))))
      (Utilities|Array|Add (Variables|Default|GetSpawnPoints) (Transformation|GetWorldTransform _returnvalue)))))

(fn SpawnObstacles
  (bind _output_get (LocalVariables|SetRandomSpawnPoints (Variables|Default|GetSpawnPoints)))
  (Utilities|Array|Shuffle _output_get)
  (for _index (range 0 (Math|Random|RandomIntegerinRange 0 2))
    (switch int (Math|Random|RandomIntegerinRange 0 1)
      (:0
        (AddComponent|AddChildActorComponent false (Math|Transform|MakeRelativeTransform (Utilities|Array|Get(acopy) (LocalVariables|GetRandomSpawnPoints) _index) (Transformation|GetActorTransform))))
      (:1
        (AddComponent|AddChildActorComponent false (Math|Transform|MakeRelativeTransform (Utilities|Array|Get(acopy) (LocalVariables|GetRandomSpawnPoints) _index) (Transformation|GetActorTransform)))))))

(fn SpawnCoins
  (for _array_element (Variables|Default|GetLanePosition)
    ;[1 1 1] Reduce coin frequency
    (for _index (range 0 9)
      (bind _returnvalue (AddComponent|AddArrowComponent false (Math|Transform|MakeTransform (Math|Vector|MakeVector (* _index 65.0) _array_element 0.0))))
      (Components|Arrow|SetArrowColor(LinearColor) _returnvalue "(R=1.000000,G=0.907290,B=0.120794,A=1.000000)")
      (Utilities|Array|Add (Variables|Default|GetCSpawn_Points) (Transformation|GetWorldTransform _returnvalue)))))

(fn CoinSpawner
  (bind _output_get (LocalVariables|SetRandomSpawnPoints (Variables|Default|GetCSpawn_Points)))
  (Utilities|Array|Shuffle _output_get)
  (for _index (range 0 (Math|Random|RandomIntegerinRange 5 8))
    (switch int 0
      (:0
        (AddComponent|AddChildActorComponent false (Math|Transform|MakeRelativeTransform (Utilities|Array|Get(acopy) (LocalVariables|GetRandomSpawnPoints) _index) (Transformation|GetActorTransform)))))))

(fn SpawnCrate
  (for _array_element (Variables|Default|GetLanePosition)
    ;[1 1 1] Reduce crate frequency
    (for _index (range 1 2)
      (bind _returnvalue (AddComponent|AddArrowComponent false (Math|Transform|MakeTransform (Math|Vector|MakeVector (* _index 275.0) _array_element 0.0))))
      (Components|Arrow|SetArrowColor(LinearColor) _returnvalue "(R=0.019147,G=0.401042,B=0.020492,A=1.000000)")
      (Utilities|Array|Add (Variables|Default|GetCrSpawn_Points) (Transformation|GetWorldTransform _returnvalue)))))

(fn CrateSpawner
  (bind _asbp_runner_game_mode (Utilities|Casting|CastToBP_RunnerGameMode (Game|GetGameMode)))
  (if (> (Variables|/Game/Runner/Blueprints/BP_RunnerGameMode.BP_RunnerGameMode_C|GetFloorCount _asbp_runner_game_mode) 5)
    (bind _output_get (LocalVariables|SetRandomSpawnPoints (Variables|Default|GetCrSpawn_Points)))
    (Utilities|Array|Shuffle _output_get)
    (switch int 0
      (:0
        (AddComponent|AddChildActorComponent false (Math|Transform|MakeRelativeTransform (Utilities|Array|Get(acopy) (LocalVariables|GetRandomSpawnPoints)) (Transformation|GetActorTransform)))
        (Variables|/Game/Runner/Blueprints/BP_RunnerGameMode.BP_RunnerGameMode_C|SetFloorCount _asbp_runner_game_mode 0)))))