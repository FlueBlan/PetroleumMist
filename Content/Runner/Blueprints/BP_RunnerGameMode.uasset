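; Game mode for an endless runner that builds the track and building scenery and loads the saved coin total.
; On BeginPlay it spawns the initial floor tiles and one building piece, reading coins from the CoinValue save slot inside the tile loop.
; Each piece spawns at the previous one's attach point.
; The Extend functions append a piece and destroy the oldest once the array exceeds its limit, keeping a rolling window.
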(event EventBeginPlay
  (Utilities|FlowControl|Sequence
    (:then_0
      (for _index (range 0 (- (Variables|Default|GetNumOfTiles) 1))
        (CallFunction|AddFloor)
        (bind _returnvalue (SaveGame|LoadGamefromSlot "CoinValue"))
        (bind _asrunner_save_game (Utilities|Casting|CastToRunner_SaveGame _returnvalue))
        (Variables|Default|SetCoins (Variables|/Game/Runner/Blueprints/Runner_SaveGame.Runner_SaveGame_C|GetCoinValue _asrunner_save_game))))
    (:then_1
      (for _index_2 (range 0 0)
        (CallFunction|AddBuildings)))))

(event EventTick
  (params (DeltaSeconds :type Float%20%28single-precision%29)))

(fn ConstructionScript)

(fn AddFloor
  (bind _returnvalue (Game|SpawnActorfromClass "/Game/Runner/Blueprints/BP_Floor.BP_Floor_C" (Variables|Default|GetFloorAttachPoint) "Undefined" "MultiplyWithRoot" 0 0))
  (bind _returnvalue_2 (Default|GetAttachPoint _returnvalue))
  (Variables|Default|SetFloorAttachPoint _returnvalue_2)
  (Utilities|Array|Add (Variables|Default|GetFloorTiles) _returnvalue)
  (bind _result (Math|Integer|IncrementInt (Variables|Default|GetFloorCount))
    (:%20%20
      (Variables|Default|SetFloorCount _result))))

(fn ExtendFloor
  (bind _floortiles (Variables|Default|GetFloorTiles))
  (bind _output (Utilities|Array|Get(acopy) _floortiles))
  (CallFunction|AddFloor)
  (if (> (Utilities|Array|Length (Variables|Default|GetFloorTiles)) (+ (Variables|Default|GetNumOfTiles) 10))
    (Actor|DestroyActor _output)
    (Utilities|Array|RemoveItem _floortiles _output)))

(fn AddBuildings
  (bind _returnvalue (Game|SpawnActorfromClass "/Game/Runner/Blueprints/BP_Buildings.BP_Buildings_C" (Variables|Default|GetBuildingSpawnPoint) "Undefined" "MultiplyWithRoot" 0 0))
  (bind _returnvalue_2 (Default|GetAttachPoint _returnvalue))
  (Variables|Default|SetBuildingSpawnPoint _returnvalue_2)
  (Utilities|Array|Add (Variables|Default|GetBP_Buildings) _returnvalue))

(fn ExtendBuildings
  (bind _bp_buildings (Variables|Default|GetBP_Buildings))
  (bind _output (Utilities|Array|Get(acopy) _bp_buildings))
  (CallFunction|AddBuildings)
  (if (> (Utilities|Array|Length (Variables|Default|GetBP_Buildings)) 8)
    (Actor|DestroyActor _output)
    (Utilities|Array|RemoveItem _bp_buildings _output)))