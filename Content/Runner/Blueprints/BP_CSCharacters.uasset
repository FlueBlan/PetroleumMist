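; Character selection Blueprint for the runner game that previews the Default, Secretary and Ronin characters and commits the chosen one.
; Show events toggle visibility so only one of the three previews is visible.
; Spawn events spawn nothing here; they pass the matching runner character as a Pawn to SaveCharacter.
; SaveCharacter loads or creates the Runner_SaveGame in the PlayerCharacter slot, stores the choice, then opens Runner_MAP.
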(event Custom|ShowRonin
  (Development|SetHiddeninGame (Variables|Default|GetSecretary) true false)
  (Development|SetHiddeninGame (Variables|Default|GetDefault) true false)
  (Development|SetHiddeninGame (Variables|Default|GetRonin) false false))

(event Custom|Show%20Secretary
  (Development|SetHiddeninGame (Variables|Default|GetSecretary) false false)
  (Development|SetHiddeninGame (Variables|Default|GetDefault) true false)
  (Development|SetHiddeninGame (Variables|Default|GetRonin) true false))

(event Custom|ShowDefault
  (Development|SetHiddeninGame (Variables|Default|GetSecretary) true false)
  (Development|SetHiddeninGame (Variables|Default|GetDefault) false false)
  (Development|SetHiddeninGame (Variables|Default|GetRonin) true false))

(event Custom|SpawnRonin
  (bind _aspawn (Utilities|Casting|CastToPawnClass "/Game/Runner/Blueprints/CharacterBPs/BP_Runner_Ronin.BP_Runner_Ronin_C"))
  (bind _output_get (Variables|Default|SetAs%20Pawn _aspawn))
  (CallFunction|SaveCharacter _output_get))

(event Custom|SpawnDefault
  (bind _aspawn (Utilities|Casting|CastToPawnClass "/Game/Runner/Blueprints/CharacterBPs/BP_RunnerCharacter.BP_RunnerCharacter_C"))
  (bind _output_get (Variables|Default|SetAs%20Pawn _aspawn))
  (CallFunction|SaveCharacter _output_get))

(event Custom|SpawnSecretary
  (bind _aspawn (Utilities|Casting|CastToPawnClass "/Game/Runner/Blueprints/CharacterBPs/BP_Runner_Secretary.BP_Runner_Secretary_C"))
  (bind _output_get (Variables|Default|SetAs%20Pawn _aspawn))
  (CallFunction|SaveCharacter _output_get))

(fn ConstructionScript)

(fn SaveCharacter
  (params (PlayerCharacter :type Pawn%20Class%20Reference))
  (bind _returnvalue (SaveGame|DoesSaveGameExist "PlayerCharacter"))
  (if _returnvalue
    (bind _returnvalue_2 (SaveGame|LoadGamefromSlot "PlayerCharacter"))
    (bind _output_get (Variables|Default|SetSaveSubClass _returnvalue_2))
    (bind _asrunner_save_game (Utilities|Casting|CastToRunner_SaveGame _output_get))
    (Variables|/Game/Runner/Blueprints/Runner_SaveGame.Runner_SaveGame_C|SetPlayerCharacter _asrunner_save_game PlayerCharacter)
    (SaveGame|SaveGametoSlot (Variables|Default|GetSaveSubClass) "PlayerCharacter")
    (else
      (bind _returnvalue_3 (SaveGame|CreateSaveGameObject "/Game/Runner/Blueprints/Runner_SaveGame.Runner_SaveGame_C"))
      (bind _output_get_2 (Variables|Default|SetSaveSubClass _returnvalue_3))
      (bind _asrunner_save_game_2 (Utilities|Casting|CastToRunner_SaveGame _output_get_2))
      (Variables|/Game/Runner/Blueprints/Runner_SaveGame.Runner_SaveGame_C|SetPlayerCharacter _asrunner_save_game_2 PlayerCharacter)
      (SaveGame|SaveGametoSlot (Variables|Default|GetSaveSubClass) "PlayerCharacter")))
  (Game|OpenLevel(byObjectReference) "/Game/Runner/Maps/Runner_MAP.Runner_MAP"))